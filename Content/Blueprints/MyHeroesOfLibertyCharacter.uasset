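; Character Blueprint for Heroes of Liberty that hooks up a debug health bar and tracks nearby targets.
; On BeginPlay it passes itself to the DEBUG_Healthbar widget held by its widget component.
; Box overlaps feed AddTargetEndOverlap, skipping itself by display-name comparison, and DeleteTargetEndOverlap on exit, both defined outside this graph.
; Hit, actor overlap and Tick events are empty, and a Swordsman_AnimationBP cast is left unconnected.
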(event `self.ReceiveBeginPlay`
  (bind _asdebug_healthbar (cast `/Game/Widgets/DEBUG_Healthbar` (`WidgetComponent.GetUserWidgetObject` (`self.DEBUG_HEALTHBAR`))))
  (set `/Game/Widgets/DEBUG_Healthbar.Character` self _asdebug_healthbar))

(event `self.ReceiveActorBeginOverlap`
  (params (OtherActor :type "Actor Object Reference")))

(event `self.Box.OnComponentHit`
  (params (HitComponent :type "PrimitiveComponent Object Reference") (OtherActor :type "Actor Object Reference") (OtherComp :type "PrimitiveComponent Object Reference") (NormalImpulse :type "Vector Structure") (Hit :type "HitResult Structure (by ref)")))

(event `self.Box.OnComponentBeginOverlap`
  (params (OverlappedComponent :type "PrimitiveComponent Object Reference") (OtherActor :type "Actor Object Reference") (OtherComp :type "PrimitiveComponent Object Reference") (OtherBodyIndex :type Integer) (bFromSweep :type Boolean) (SweepResult :type "HitResult Structure (by ref)"))
  (if (`KismetStringLibrary.NotEqual_StrStr` (`KismetSystemLibrary.GetDisplayName` OtherActor) (`KismetSystemLibrary.GetDisplayName` self))
    (`self.AddTargetEndOverlap` OtherActor)))

(event `self.Box.OnComponentEndOverlap`
  (params (OverlappedComponent :type "PrimitiveComponent Object Reference") (OtherActor :type "Actor Object Reference") (OtherComp :type "PrimitiveComponent Object Reference") (OtherBodyIndex :type Integer))
  (`self.DeleteTargetEndOverlap` OtherActor))

(fn `UserConstructionScript`)