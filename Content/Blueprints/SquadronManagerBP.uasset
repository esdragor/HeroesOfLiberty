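; Squadron manager Blueprint that spawns a requested number of soldiers from a starting position.
; SpawnUnitsBP spawns actors of the passed object's class in a latent loop with a short delay after each, adjusting for collisions but always spawning.
; Each soldier goes through SetValueNewSoldier, then UpdateSpawnPos moves the position until the count is reached and FinishSpawningSoldier runs.
; The count is checked after spawning, so at least one soldier always spawns.
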(event `self.SpawnUnitsBP`
  (params (nb :type Integer) (objToSpawn :type "HeroesOfLibertyCharacter Object Reference") (pos :type "Vector Structure"))
  (set `self.Position` pos)
  (set `self.cpt` 0)
  (set `self.MaxSpawn` nb)
  (set `self.ActorToSpaw` objToSpawn)
  (bind _returnvalue (`|SpawnActorFromClass` (`GameplayStatics.GetObjectClass` (`self.ActorToSpaw`)) (`KismetMathLibrary.MakeTransform` (`self.Position`)) "AdjustIfPossibleButAlwaysSpawn" "OverrideRootScale" null null :!label _label))
  (`KismetSystemLibrary.Delay` 0.2)
  (`self.SetValueNewSoldier` _returnvalue)
  (`/Engine/EditorBlueprintResources/StandardMacros.IncrementInt` (`self.cpt`)
    (:`  `
      (bind _needspawning (`self.NeedNewSpawn`))
      (if _needspawning
        (bind _returnvalue_2 (`self.UpdateSpawnPos` (`self.cpt`) (`self.MaxSpawn`) (`self.Position`)))
        (set `self.Position` _returnvalue_2)
        (goto _label)
        (else
          (`self.FinishSpawningSoldier`))))))

(fn `NeedNewSpawn`
  (returns (NeedSpawning :type Boolean))
  (return (< (`self.cpt`) (`self.MaxSpawn`))))

(fn `UserConstructionScript`)